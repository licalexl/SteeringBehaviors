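; Wandering actor, filed under the steering behavior targets, that roams between random points in a box around a fixed origin.
; BeginPlay picks the first Destino; Tick steps forward by Velocidad per frame, not delta-scaled, while RInterpTo turns it toward Destino.
; On arrival it stops if PararMovimiento is set, otherwise retargets; while farther away, a Delay of TiempoDeDireccion also retargets.
; Retargeting uses X for both horizontal extents, unlike BeginPlay.
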(event EventBeginPlay
  ;[1 1 1] Crear Destino Random Al iniciar
  (Variables|Default|SetDestino (Math|Random|RandomPointinBoundingBox "0, 0,50.000000" (Math|Vector|MakeVector (Variables|Wander|GetX) (Variables|Wander|GetY) (Variables|Wander|GetZ)))))

(event EventTick
  (params (DeltaSeconds :type Float%20%28single-precision%29))
  ;[1 1 1 1 11] Condición: Este pin toma un valor booleano como entrada. Si el valor es true, se ejecutan los nodos conectados al pin Ejecutar si verdadero. Si el valor es false, se ejecutan los nodos conectados al pin Ejecutar si falso.
  (if true
    ;[1 1 1 1 12] serie de eventos que se ejecutan en orden específico. Cada evento puede ser una acción, un efecto visual, una condición o una combinación de estos. Los eventos se pueden conectar entre sí para crear flujos de trabajo complejos y animaciones dinámicas.
    (Utilities|FlowControl|Sequence
      (:then_0
        ;[1 1 1 1 12] La función Set Actor Location and Rotation toma dos entradas principales:
        ;
        ; Nueva ubicación: Este pin toma un vector que especifica la nueva posición del actor en el mundo.
        ;
        ; Nueva rotación: Este pin toma un rotador que especifica la nueva orientación del actor en el mundo.
        (Transformation|SetActorLocationAndRotation (+ (Transformation|GetActorLocation) (* (Transformation|GetActorForwardVector) (Variables|Wander|GetVelocidad))) (Math|Interpolation|RInterpTo (Transformation|GetActorRotation) (Math|Rotator|FindLookatRotation (Transformation|GetActorLocation) (Variables|Default|GetDestino)) (Utilities|Time|GetWorldDeltaSeconds) 5.0)))
      (:then_1
        (if (<= (Math|Vector|Distance(Vector) (Transformation|GetActorLocation) (Variables|Default|GetDestino)) 5e+01)
          (if (Variables|Wander|GetPararMovimiento)
            (Variables|Wander|SetVelocidad 0.0)
            (else
              (Variables|Default|SetDestino (Math|Random|RandomPointinBoundingBox "0, 0,50.000000" (Math|Vector|MakeVector (Variables|Wander|GetX) (Variables|Wander|GetX) (Variables|Wander|GetZ))) :!label _label)
              (Variables|Wander|SetVelocidad 1e+01)))
          (else
            (Utilities|FlowControl|Delay (Variables|Wander|GetTiempoDeDireccion))
            (goto _label)))))))

(fn ConstructionScript)