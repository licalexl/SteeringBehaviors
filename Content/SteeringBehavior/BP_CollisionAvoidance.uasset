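; Steering-behavior actor that seeks the nearest target while turning away from nearby obstacles, with a static mesh added at construction.
; BeginPlay gathers targets and obstacles by class, re-adding the obstacles for every target found.
; Each Tick, Seek moves it forward, slows it within braking range and interpolates rotation toward the closest target.
; Esquivar then steers away from close obstacles using look-at between negated positions; an eight-direction line trace is unconnected.
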(event EventBeginPlay
  (for _array_element (Variables|CollisionAvoidance|GetTarget)
    ;[1 1 1 1 12] devuelve el valor mínimo en una matriz  flotante. y  proporciona el índice del elemento en la matriz que contiene el valor mínimo.
    (bind _outactors (Actor|GetAllActorsOfClass _array_element))
    (for _array_element_2 _outactors
      (Utilities|Array|Add (Variables|Default|GetArrival_Target) _array_element_2)
      (for _array_element_3 (Variables|CollisionAvoidance|GetObjetivosOBSTACULOS)
        (bind _outactors_2 (Actor|GetAllActorsOfClass _array_element_3))
        (for _array_element_4 _outactors_2
          (Utilities|Array|Add (Variables|Default|GetOBSTarget) _array_element_4))))))

(event EventTick
  (params (DeltaSeconds :type Float%20%28single-precision%29))
  (Utilities|FlowControl|Sequence
    (:then_0
      (CallFunction|Seek))
    (:then_1
      (CallFunction|Esquivar))))

(fn ConstructionScript
  (bind _returnvalue (AddComponent|AddStaticMeshComponent false (Math|Transform|MakeTransform "0, 0,-50.000000" "0, 0, 0" "1,1,1")))
  (Components|StaticMesh|SetStaticMesh _returnvalue (Variables|CollisionAvoidance|GetStaticMesh)))

(fn Seek
  (Utilities|FlowControl|Sequence
    (:then_0
      (Transformation|AddActorLocalOffset (Math|Vector|MakeVector (Variables|CollisionAvoidance|GetVelocidad) 0.0 0.0) false false))
    (:then_1
      (if (Variables|CollisionAvoidance|GetTerminarObjetivo)
        (for (_array_element _array_index) (Variables|Default|GetArrival_Target)
          ;[1 1 1 1 12] establecer el valor de un elemento específico en una matriz. La función toma tres entradas principales:
          ;
          ; Array: Este pin especifica la matriz en la que se va a establecer el valor.
          ; Index: Este pin especifica el índice del elemento en la matriz que se va a establecer.
          ; Value: Este pin especifica el nuevo valor del elemento.
          ; La función establece el valor del elemento en la matriz especificada en el índice especificado con el nuevo valor especificado.
          (Utilities|Array|SetArrayElem (Variables|Default|GetTargetDistance) _array_index (Transformation|GetDistanceTo _array_element) true)
          (if (> (Transformation|GetDistanceTo _array_element) (Variables|CollisionAvoidance|GetdistanciaDeFrenado))
            _
            (elif (> (Transformation|GetDistanceTo _array_element) (Variables|CollisionAvoidance|GetdistanciaDeParado))
              (Variables|CollisionAvoidance|SetVelocidad (/ (Transformation|GetDistanceTo _array_element) (Variables|CollisionAvoidance|GetFuerzaDeFrenado)))
              (else
                (Variables|CollisionAvoidance|SetVelocidad 0.0))))
          (Transformation|SetActorRotation (Math|Interpolation|RInterpTo (Transformation|GetActorRotation) (Math|Rotator|FindLookatRotation (Transformation|GetActorLocation) (Transformation|GetActorLocation (Utilities|Array|Get(acopy) (Variables|Default|GetArrival_Target) (.IndexOfMinValue (Math|Float|MinOfFloatArray (Variables|Default|GetTargetDistance)))))) (Utilities|Time|GetWorldDeltaSeconds) 5.0)))
        (else
          (if (> (Transformation|GetDistanceTo _array_element) (Variables|CollisionAvoidance|GetdistanciaDeFrenado))
            _
            (elif (> (Transformation|GetDistanceTo _array_element) (Variables|CollisionAvoidance|GetdistanciaDeParado))
              (Variables|CollisionAvoidance|SetVelocidad (/ (Transformation|GetDistanceTo _array_element) (Variables|CollisionAvoidance|GetFuerzaDeFrenado)))
              (else
                (Variables|CollisionAvoidance|SetVelocidad 0.0))))
          (Transformation|SetActorRotation (Math|Interpolation|RInterpTo (Transformation|GetActorRotation) (Math|Rotator|FindLookatRotation (Transformation|GetActorLocation) (Transformation|GetActorLocation (Utilities|Array|Get(acopy) (Variables|Default|GetArrival_Target) (.IndexOfMinValue (Math|Float|MinOfFloatArray (Variables|Default|GetTargetDistance)))))) (Utilities|Time|GetWorldDeltaSeconds) 5.0)))))))

(fn Esquivar
  (if (Variables|CollisionAvoidance|GetExisteObstaculo)
    (for (_ _array_index) (Variables|Default|GetOBSTarget)
      (if (< (Transformation|GetDistanceTo (Utilities|Array|Get(acopy) (Variables|Default|GetOBSTarget) _array_index)) (Variables|CollisionAvoidance|GetDistanciaEsquivar))
        (Transformation|SetActorRotation (Math|Interpolation|RInterpTo (Transformation|GetActorRotation) (Math|Rotator|FindLookatRotation (Math|Vector|NegateVector (Transformation|GetActorLocation)) (Math|Vector|NegateVector (Transformation|GetActorLocation (Utilities|Array|Get(acopy) (Variables|Default|GetOBSTarget) _array_index)))) (Utilities|Time|GetWorldDeltaSeconds) 3.0))))
    (else
      (if (< (Transformation|GetDistanceTo (Utilities|Array|Get(acopy) (Variables|Default|GetOBSTarget) _array_index)) (Variables|CollisionAvoidance|GetDistanciaEsquivar))
        (Transformation|SetActorRotation (Math|Interpolation|RInterpTo (Transformation|GetActorRotation) (Math|Rotator|FindLookatRotation (Math|Vector|NegateVector (Transformation|GetActorLocation)) (Math|Vector|NegateVector (Transformation|GetActorLocation (Utilities|Array|Get(acopy) (Variables|Default|GetOBSTarget) _array_index)))) (Utilities|Time|GetWorldDeltaSeconds) 3.0))))))