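; Steering-behavior Arrival actor that moves along its local X by Velocidad each tick and turns toward the nearest recorded target.
; BeginPlay gathers targets from the classes in Objeto, and the construction script adds its mesh.
; While ObjetivoTerminado is true, Tick refreshes the distance array used to choose the facing target.
; Distance thresholds are meant to brake then stop, but both set speed to zero because braking divides zero by FuerzaDeFrenado.
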(event EventBeginPlay
  ;[1 1 1 1 12] un bucle en Unreal Engine Blueprints que se utiliza para iterar sobre una colección de elementos y ejecutar un conjunto de acciones para cada elemento. La colección de elementos puede ser un arreglo, una secuencia o cualquier otro tipo de contenedor que admita la iteración.
  (for _array_element (Variables|Arrival|GetObjeto)
    ;[1 1 1 1 12] se utiliza para obtener una lista de todos los actores de una clase específica que existen actualmente en el mundo del juego. La función toma una entrada principal:
    ;
    ; Class: Este pin especifica la clase de actores que se desea obtener.
    ; La función devuelve una matriz que contiene referencias a todos los actores de la clase especificada que se encontraron en el mundo del juego.
    (bind _outactors (Actor|GetAllActorsOfClass _array_element))
    (for _array_element_2 _outactors
      (Utilities|Array|Add (Variables|Default|GetObjetoArrival) _array_element_2))))

(event EventTick
  (params (DeltaSeconds :type Float%20%28single-precision%29))
  (Utilities|FlowControl|Sequence
    (:then_0
      ;[1 1 1] es una función se utiliza para agregar un desplazamiento local a la ubicación y rotación de un actor. Un desplazamiento local es un cambio en la posición o la orientación del actor en relación con su ubicación y orientación actuales.
      (Transformation|AddActorLocalOffset (Math|Vector|MakeVector (Variables|Arrival|GetVelocidad) 0.0 0.0) false false))
    (:then_1
      (Transformation|SetActorRotation (Math|Interpolation|RInterpTo (Transformation|GetActorRotation) (Math|Rotator|FindLookatRotation (Transformation|GetActorLocation) (Transformation|GetActorLocation (Utilities|Array|Get(acopy) (Variables|Default|GetObjetoArrival) (.IndexOfMinValue (Math|Float|MinOfFloatArray (Variables|Default|GetDistanciaParaArrival)))))) (Utilities|Time|GetWorldDeltaSeconds) 5.0)))
    (:then_2
      (if (Variables|Arrival|GetObjetivoTerminado)
        (for (_array_element _array_index) (Variables|Default|GetObjetoArrival)
          ;[1 1 1 1 12] establecer el valor de un elemento específico en una matriz. La función toma tres entradas principales:
          ;
          ; Array: Este pin especifica la matriz en la que se va a establecer el valor.
          ; Index: Este pin especifica el índice del elemento en la matriz que se va a establecer.
          ; Value: Este pin especifica el nuevo valor del elemento.
          ; La función establece el valor del elemento en la matriz especificada en el índice especificado con el nuevo valor especificado.
          (Utilities|Array|SetArrayElem (Variables|Default|GetDistanciaParaArrival) _array_index (Transformation|GetDistanceTo _array_element) true)
          (if (> (Transformation|GetDistanceTo _array_element) (Variables|Arrival|GetPerderVelocidadDistanciaMin))
            (Variables|Arrival|SetVelocidad (Variables|Arrival|GetVelocidad))
            (elif (> (Transformation|GetDistanceTo _array_element) (Variables|Arrival|GetDistanciaDeParado))
              (Variables|Arrival|SetVelocidad (/ 0.0 (Variables|Arrival|GetFuerzaDeFrenado)))
              (else
                (Variables|Arrival|SetVelocidad 0.0)))))
        (else
          (if (> (Transformation|GetDistanceTo _array_element) (Variables|Arrival|GetPerderVelocidadDistanciaMin))
            (Variables|Arrival|SetVelocidad (Variables|Arrival|GetVelocidad))
            (elif (> (Transformation|GetDistanceTo _array_element) (Variables|Arrival|GetDistanciaDeParado))
              (Variables|Arrival|SetVelocidad (/ 0.0 (Variables|Arrival|GetFuerzaDeFrenado)))
              (else
                (Variables|Arrival|SetVelocidad 0.0)))))))))

(fn ConstructionScript
  (bind _returnvalue (AddComponent|AddStaticMeshComponent false (Math|Transform|MakeTransform "0, 0,-50.000000" "0, 0, 0" "1,1,1")))
  (Components|StaticMesh|SetStaticMesh _returnvalue (Variables|Arrival|GetStaticMesh)))