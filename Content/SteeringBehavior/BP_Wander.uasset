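; Wander steering behavior actor that roams toward random points inside a box near the world origin.
; Each Tick it moves along local X by Velocidad, unscaled by delta time, and smoothly interpolates its rotation toward Destino.
; It picks a new destination on arrival, or stops if Paso is set; while en route, a Delay also renews the destination periodically.
; The construction script adds the configurable static mesh.
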(event EventBeginPlay
  ;[1 1 1] Copia de Primer Codigo solo para diambular
  (Variables|Components|SetDestino (Math|Random|RandomPointinBoundingBox "0, 0,50.000000" (Math|Vector|MakeVector (Variables|Components|GetX) (Variables|Components|GetY) (Variables|Components|GetZ)))))

(event EventTick
  (params (DeltaSeconds :type Float%20%28single-precision%29))
  ;[1 1 1] Copia de Primer Codigo solo para diambular
  (Utilities|FlowControl|Sequence
    (:then_0
      ;[1 1 1] es una función se utiliza para agregar un desplazamiento local a la ubicación y rotación de un actor. Un desplazamiento local es un cambio en la posición o la orientación del actor en relación con su ubicación y orientación actuales.
      (Transformation|AddActorLocalOffset (Math|Vector|MakeVector (Variables|Components|GetVelocidad) 0.0 0.0) false false))
    (:then_1
      (Transformation|SetActorRotation (Math|Interpolation|RInterpTo (Transformation|GetActorRotation) (Math|Rotator|FindLookatRotation (Transformation|GetActorLocation) (Variables|Components|GetDestino)) (Utilities|Time|GetWorldDeltaSeconds) 5.0)))
    (:then_2
      (if (<= (Math|Vector|Distance(Vector) (Transformation|GetActorLocation) (Variables|Components|GetDestino)) 1e+02)
        (if (Variables|Components|GetPaso)
          (Variables|Components|SetVelocidad 0.0)
          (else
            (Variables|Components|SetDestino (Math|Random|RandomPointinBoundingBox "0, 0,50.000000" (Math|Vector|MakeVector (Variables|Components|GetX) (Variables|Components|GetY) (Variables|Components|GetZ))) :!label _label)
            (Variables|Components|SetVelocidad 1e+01)))
        (else
          (Utilities|FlowControl|Delay (Variables|Components|GetTiempoRenovarDireccion))
          (goto _label))))))

(fn ConstructionScript
  (bind _returnvalue (AddComponent|AddStaticMeshComponent false (Math|Transform|MakeTransform "0, 0,-50.000000" "0, 0, 0" "1,1,1")))
  (Components|StaticMesh|SetStaticMesh _returnvalue (Variables|Components|GetStaticMesh)))