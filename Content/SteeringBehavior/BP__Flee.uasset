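; Steering-behavior actor that flees from instances of the classes listed in Target, gathered into FleeTarget at BeginPlay.
; Each Tick, targets closer than DistanciaMinimaEffecto trigger a delayed local forward step of DistanciaMinima and an interpolated turn away, using look-at on negated positions.
; With ObjetoFlee off, Tick still enters that distance check, bypassing the loop.
; The construction script adds the configurable, lowered static mesh.
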(event EventBeginPlay
  ;[1 1 1 1 12] un bucle en Unreal Engine Blueprints que se utiliza para iterar sobre una colección de elementos y ejecutar un conjunto de acciones para cada elemento. La colección de elementos puede ser un arreglo, una secuencia o cualquier otro tipo de contenedor que admita la iteración.
  (for _array_element (Variables|Components|GetTarget)
    ;[1 1 1 1 12] se utiliza para obtener una lista de todos los actores de una clase específica que existen actualmente en el mundo del juego. La función toma una entrada principal:
    ;
    ; Class: Este pin especifica la clase de actores que se desea obtener.
    ; La función devuelve una matriz que contiene referencias a todos los actores de la clase especificada que se encontraron en el mundo del juego.
    (bind _outactors (Actor|GetAllActorsOfClass _array_element))
    (for _array_element_2 _outactors
      ;[1 1 1 1 12] Comment
      (Utilities|Array|Add (Variables|Components|GetFleeTarget) _array_element_2))))

(event EventTick
  (params (DeltaSeconds :type Float%20%28single-precision%29))
  (if (Variables|Components|GetObjetoFlee)
    (for (_array_element _array_index) (Variables|Components|GetFleeTarget)
      ;[1 1 1] Defines a minimum distance between Static Mesh and Target
      (if (< (Transformation|GetDistanceTo _array_element) (Variables|Components|GetDistanciaMinimaEffecto))
        (Utilities|FlowControl|Sequence
          (:then_0
            ;[1 1 1] This sets the Static Mesh to move 5 units forward
            (Utilities|FlowControl|Delay (Utilities|Time|GetWorldDeltaSeconds))
            (Transformation|AddActorLocalOffset (Math|Vector|MakeVector (Variables|Components|GetDistanciaMinima) 0.0 0.0) false false))
          (:then_1
            (Transformation|SetActorRotation (Math|Interpolation|RInterpTo (Transformation|GetActorRotation) (Math|Rotator|FindLookatRotation (Math|Vector|NegateVector (Transformation|GetActorLocation)) (Math|Vector|NegateVector (Transformation|GetActorLocation (Utilities|Array|Get(acopy) (Variables|Components|GetFleeTarget) _array_index)))) (Utilities|Time|GetWorldDeltaSeconds) 5.0))))))
    (else
      (if (< (Transformation|GetDistanceTo _array_element) (Variables|Components|GetDistanciaMinimaEffecto))
        (Utilities|FlowControl|Sequence
          (:then_0
            (Utilities|FlowControl|Delay (Utilities|Time|GetWorldDeltaSeconds))
            (Transformation|AddActorLocalOffset (Math|Vector|MakeVector (Variables|Components|GetDistanciaMinima) 0.0 0.0) false false))
          (:then_1
            (Transformation|SetActorRotation (Math|Interpolation|RInterpTo (Transformation|GetActorRotation) (Math|Rotator|FindLookatRotation (Math|Vector|NegateVector (Transformation|GetActorLocation)) (Math|Vector|NegateVector (Transformation|GetActorLocation (Utilities|Array|Get(acopy) (Variables|Components|GetFleeTarget) _array_index)))) (Utilities|Time|GetWorldDeltaSeconds) 5.0))))))))

(fn ConstructionScript
  (bind _returnvalue (AddComponent|AddStaticMeshComponent false (Math|Transform|MakeTransform "0, 0,-50.000000" "0, 0, 0" "1,1,1")))
  (Components|StaticMesh|SetStaticMesh _returnvalue (Variables|Components|GetStaticMesh)))